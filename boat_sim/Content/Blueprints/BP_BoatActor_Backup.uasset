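; BP_BoatActor_Backup is a boat actor that passes player throttle and rudder input to a boat movement component.
; On BeginPlay it looks up its BoatMovementComponent and, if found, adds the IMC_Boat Enhanced Input context for player 0.
; Throttle and rudder actions print their values and forward them to the component, resetting to zero on completion.
; A SetViewTargetWithBlend node is left unconnected, and overlap and Tick events are empty.
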(event `EnhancedInput|/Game/Input/IA_Throttle`
  (params (ActionValue :type "Float (double-precision)") (ElapsedSeconds :type "Float (double-precision)") (TriggeredSeconds :type "Float (double-precision)") (InputAction :type "InputAction Object Reference" :default "/Game/Input/IA_Throttle.IA_Throttle"))
  (bind _boatmovementref (`self.BoatMovementRef`))
  (:`Triggered`
    (`KismetSystemLibrary.PrintString` (`KismetStringLibrary.Conv_DoubleToString` ActionValue))
    (`BoatMovementComponent.SetThrottle` _boatmovementref ActionValue))
  (:`Completed`
    (`BoatMovementComponent.SetThrottle` _boatmovementref 0.0)))

(event `self.ReceiveBeginPlay`
  (bind _output_get (set `self.BoatMovementRef` (`self.GetComponentByClass` "/Script/boat_sim.BoatMovementComponent")))
  (`/Engine/EditorBlueprintResources/StandardMacros.IsValid` _output_get
    (:`Is Valid`
      (`EnhancedInputSubsystemInterface.AddMappingContext` (pcsubsystem `EnhancedInputLocalPlayerSubsystem` (`GameplayStatics.GetPlayerController` 0)) "/Game/Input/IMC_Boat.IMC_Boat" 0 (struct)))
    (:`Is Not Valid`
      (`KismetSystemLibrary.PrintString` "Movement Not Found"))))

(event `EnhancedInput|/Game/Input/IA_Rudder`
  (params (ActionValue :type "Float (double-precision)") (ElapsedSeconds :type "Float (double-precision)") (TriggeredSeconds :type "Float (double-precision)") (InputAction :type "InputAction Object Reference" :default "/Game/Input/IA_Rudder.IA_Rudder"))
  (bind _boatmovementref (`self.BoatMovementRef`))
  (:`Triggered`
    (`KismetSystemLibrary.PrintString` (`KismetStringLibrary.Conv_DoubleToString` ActionValue))
    (`BoatMovementComponent.SetRudder` _boatmovementref ActionValue))
  (:`Completed`
    (`BoatMovementComponent.SetRudder` _boatmovementref 0.0)))

(fn `UserConstructionScript`)