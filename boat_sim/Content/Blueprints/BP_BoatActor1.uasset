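; BP_BoatActor1 is a player-controlled boat actor driven through Enhanced Input.
; BeginPlay adds the IMC_Boat mapping context to the first player controller's input subsystem.
; Throttle and rudder actions print their values and pass them to MovementComponent, resetting to zero when input completes.
; Unconnected leftover nodes hold a movement-component lookup and a view-target switch, neither of which runs.
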(event `self.ReceiveBeginPlay`
  (`EnhancedInputSubsystemInterface.AddMappingContext` (pcsubsystem `EnhancedInputLocalPlayerSubsystem` (`GameplayStatics.GetPlayerController` 0)) "/Game/Input/IMC_Boat.IMC_Boat" 0 (struct)))

(event `EnhancedInput|/Game/Input/IA_Throttle`
  (params (ActionValue :type "Float (double-precision)") (ElapsedSeconds :type "Float (double-precision)") (TriggeredSeconds :type "Float (double-precision)") (InputAction :type "InputAction Object Reference" :default "/Game/Input/IA_Throttle.IA_Throttle"))
  (bind _movementcomponent (`self.MovementComponent`))
  (:`Triggered`
    (`KismetSystemLibrary.PrintString` (`KismetStringLibrary.Conv_DoubleToString` ActionValue))
    (`BoatMovementComponent.SetThrottle` _movementcomponent ActionValue))
  (:`Completed`
    (`BoatMovementComponent.SetThrottle` _movementcomponent 0.0)))

(event `EnhancedInput|/Game/Input/IA_Rudder`
  (params (ActionValue :type "Float (double-precision)") (ElapsedSeconds :type "Float (double-precision)") (TriggeredSeconds :type "Float (double-precision)") (InputAction :type "InputAction Object Reference" :default "/Game/Input/IA_Rudder.IA_Rudder"))
  (bind _movementcomponent (`self.MovementComponent`))
  (:`Triggered`
    (`KismetSystemLibrary.PrintString` (`KismetStringLibrary.Conv_DoubleToString` ActionValue))
    (`BoatMovementComponent.SetRudder` _movementcomponent ActionValue))
  (:`Completed`
    (`BoatMovementComponent.SetRudder` _movementcomponent 0.0)))

(fn `UserConstructionScript`)